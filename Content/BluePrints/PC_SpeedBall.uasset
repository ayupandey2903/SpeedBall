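; PC_SpeedBall is the player controller that rolls the player's ball and manages the main and win screens.
; MoveForward and MoveRight axis input fetch the ball from the pawn via GetBallRefMessage and apply scaled torque as acceleration, ignoring mass.
; BeginPlay shows the WB_Main widget, and DisplayWinUI swaps it for WB_Win.
; GetPlayerControllerRef returns the controller itself.
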(event `self.ReceiveBeginPlay`
  (bind _returnvalue (`|CreateWidget` "/Game/UI/WB_Main.WB_Main_C"))
  (bind _output_get (set `self.WB_Main` _returnvalue))
  (`UserWidget.AddToViewport` _output_get 0))

(event `InputAxis|MoveForward`
  (params (AxisValue :type "Float (single-precision)"))
  (bind _ball (message `/Game/BluePrints/InterFaces/INT_BPBall.GetBallRef` (`GameplayStatics.GetPlayerPawn` 0)))
  (bind _ball_2 (`/Game/BluePrints/BP_Ball.Ball` _ball)
    (:`then`
      (`PrimitiveComponent.AddTorqueInRadians` _ball_2 (`KismetMathLibrary.MakeVector` (* AxisValue 35.0)) "None" true))
    (:`else`)))

(event `InputAxis|MoveRight`
  (params (AxisValue :type "Float (single-precision)"))
  (bind _ball (message `/Game/BluePrints/InterFaces/INT_BPBall.GetBallRef` (`GameplayStatics.GetPlayerPawn` 0)))
  (bind _ball_2 (`/Game/BluePrints/BP_Ball.Ball` _ball)
    (:`then`
      (`PrimitiveComponent.AddTorqueInRadians` _ball_2 (`KismetMathLibrary.MakeVector` 0.0 (* AxisValue 35.0)) "None" true))
    (:`else`)))

(event `/Game/BluePrints/InterFaces/INT_PlayerController.DisplayWinUI`
  (`Widget.RemoveFromParent` (`self.WB_Main`))
  (bind _returnvalue (`|CreateWidget` "/Game/UI/WB_Win.WB_Win_C"))
  (`UserWidget.AddToViewport` _returnvalue 0))

(fn `GetPlayerControllerRef`
  (returns (PlayerController :type "/Game/BluePrints/PC_SpeedBall Object Reference"))
  (return self))

(fn `UserConstructionScript`)