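; BP_Star is a collectible star pickup that animates along its local X axis while idle.
; When a Player-tagged actor overlaps TriggerSphere, it reports the star to the game mode via a message call and plays a 2D sound.
; It then hides PStar and runs a loot timeline that adds X offsets cumulatively to the current location and drives yaw, destroying the actor when finished.
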(event `self.ReceiveBeginPlay`
  (bind (_direction _locationalpha) (`Timeline|StarMovement`)
    (:`Update`
      (`SceneComponent.K2_SetRelativeLocation` (`self.Star`) (`KismetMathLibrary.MakeVector` (.x _locationalpha)) false false))))

(event `self.TriggerSphere.OnComponentBeginOverlap`
  (params (OverlappedComponent :type "PrimitiveComponent Object Reference") (OtherActor :type "Actor Object Reference") (OtherComp :type "PrimitiveComponent Object Reference") (OtherBodyIndex :type Integer) (bFromSweep :type Boolean) (SweepResult :type "HitResult Structure (by ref)"))
  (if (`self.ActorHasTag` OtherActor "Player")
    (bind _gamemode (message `/Game/BluePrints/InterFaces/INT_GAME.GetGameModRef` (`GameplayStatics.GetGameMode`)))
    (message `/Game/BluePrints/InterFaces/INT_GAME.AddStar` _gamemode)
    (`self.StarLooted`)
    (`GameplayStatics.PlaySound2D` "/Game/Audio/SC_Star.SC_Star" 1.0 1.0 0.0 null null)))

(event `StarLooted`
  (bind (_returnvalue_x _returnvalue_y _returnvalue_z) (`KismetMathLibrary.BreakVector` (`self.K2_GetActorLocation`)))
  (bind (_returnvalue_roll _returnvalue_pitch) (`KismetMathLibrary.BreakRotator` (`self.K2_GetActorRotation`)))
  (`SceneComponent.SetVisibility` (`self.P_Star`) false false)
  (bind (_direction _locationalpha _rotationalpha) (`Timeline|StarLootMovement`)
    (:`Update`
      (`self.K2_SetActorRelativeLocation` (`KismetMathLibrary.MakeVector` (+ _returnvalue_x (.x _locationalpha)) _returnvalue_y _returnvalue_z))
      (`self.K2_SetActorRelativeRotation` (`KismetMathLibrary.MakeRotator` _returnvalue_roll _returnvalue_pitch _rotationalpha)))
    (:`Finished`
      (`self.K2_DestroyActor`))))

(fn `UserConstructionScript`)